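; BP_EnemyCharge is an enemy bot that runs at a player character it spots.
; When PawnSensing sees a ThirdPersonCharacter and the bot is not dead, AIMoveTo moves it toward that target.
; Arrival prints a debug message and raises the Attacking flag, which a one-shot timer clears shortly after.
; A failed move also clears the flag; no damage is applied in this graph.
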(event OnSeePawn(PawnSensing)
  (params (Pawn :type Pawn%20Object%20Reference))
  (if (not (Variables|Default|GetIsDead))
    (bind _asthird_person_character (Utilities|Casting|CastToThirdPersonCharacter Pawn))
    (AI|AIMoveTo self "0, 0, 0" _asthird_person_character 1e+02 false
      (:OnSuccess
        (Development|PrintString "Doszedł")
        (Variables|Default|SetAttacking true)
        (Utilities|Time|SetTimerbyEvent (delegate Custom|CustomEvent_0) 1.0))
      (:OnFail
        (if (Variables|Default|GetAttacking)
          (Variables|Default|SetAttacking false))))))

(event Custom|CustomEvent_0
  (Variables|Default|SetAttacking false))

(fn ConstructionScript
  (|CallParentFunction))