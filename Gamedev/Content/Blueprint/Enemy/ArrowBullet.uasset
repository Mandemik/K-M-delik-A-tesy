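; ArrowBullet is an enemy projectile actor, apparently fired by a turret.
; Each tick it moves along its forward vector by SpeedMove without sweep or delta-time scaling, so its speed depends on frame rate.
; When its capsule overlaps anything other than itself or its Turret, it calls PlayerGotHit on a ThirdPersonCharacter, prints the hit actor's name and destroys itself.
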(event OnComponentBeginOverlap(Capsule)
  (params (OverlappedComponent :type Primitive%20Component%20Object%20Reference) (OtherActor :type Actor%20Object%20Reference) (OtherComp :type Primitive%20Component%20Object%20Reference) (OtherBodyIndex :type Integer) (bFromSweep :type Boolean) (SweepResult :type Hit%20Result%20Structure%20%28by%20ref%29))
  (if (not (or (== OtherActor self) (== OtherActor (Variables|Default|GetTurret))))
    (Utilities|FlowControl|Sequence
      (:then_0
        (bind _asthird_person_character (Utilities|Casting|CastToThirdPersonCharacter OtherActor))
        (Default|PlayerGotHit _asthird_person_character))
      (:then_1
        (Development|PrintString (Utilities|GetDisplayName OtherActor)))
      (:then_2
        (Actor|DestroyActor)))))

(event EventTick
  (params (DeltaSeconds :type Float%20%28single-precision%29))
  (Transformation|SetActorLocation (+ (Transformation|GetActorLocation) (* (Transformation|GetActorForwardVector) (Variables|Default|GetSpeedMove))) false false))

(fn ConstructionScript)