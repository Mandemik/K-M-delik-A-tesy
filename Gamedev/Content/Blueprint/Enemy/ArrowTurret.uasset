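; ArrowTurret is an enemy turret that fires projectiles at a fixed interval.
; On BeginPlay it fires once, then starts a looping timer based on Frequency, presumably bound to CreatBullet.
; CreatBullet spawns a BulletClass actor at the SpawnBulletPlace transform, passing it the bullet speed and a reference to the turret.
; It has no aiming or targeting logic in its graphs.
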(event Custom|CreatBullet
  (Game|SpawnActorfromClass (Variables|Default|GetBulletClass) (Transformation|GetWorldTransform (Variables|Default|GetSpawnBulletPlace)) "Undefined" 0 (Variables|Default|GetSpeedBullet) self 0))

(event EventBeginPlay
  (CallFunction|CreatBullet)
  (Utilities|Time|SetTimerbyEvent (EventDispatchers|CreateEvent :!event Custom|CreatBullet) (Variables|Default|GetFrequency) true))

(fn ConstructionScript)