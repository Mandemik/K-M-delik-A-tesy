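; PickableItem is a pickup actor that gives the player a back bag or one-hand weapon, then destroys itself.
; On BeginPlay, a looping timeline drives the yaw of its scene component.
; ItemPicked switches on ItemType, looks up RowName in the matching GamedecGM data table, and passes the type, mesh and material to the player's PickUpItem.
; Both item types read the BagMesh and BagMaterial row fields.
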(event Custom|ItemPicked
  (switch Utilities|FlowControl|Switch|SwitchonItemType (Variables|Default|GetItem%20Type)
    (:NewEnumerator0
      (bind _returnvalue (Utilities|GetDataTableRow (Variables|/Game/Blueprint/GamedecGM.GamedecGM_C|GetBackBackDataTable (.AsGamedec%20GM (Utilities|Casting|CastToGamedecGM (Game|GetGameMode)))) (Variables|Default|GetRowName))
        (:then
          (Default|PickUpItem (Variables|Default|GetPlayer) (Variables|Default|GetItem%20Type) (.BagMesh (Utilities|Struct|BreakItemStruct _returnvalue)) (.BagMaterial (Utilities|Struct|BreakItemStruct _returnvalue))))))
    (:NewEnumerator1
      (bind _returnvalue_2 (Utilities|GetDataTableRow (Variables|/Game/Blueprint/GamedecGM.GamedecGM_C|GetOneWeaponDataTable (.AsGamedec%20GM (Utilities|Casting|CastToGamedecGM (Game|GetGameMode)))) (Variables|Default|GetRowName))
        (:then
          (Default|PickUpItem (Variables|Default|GetPlayer) (Variables|Default|GetItem%20Type) (.BagMesh (Utilities|Struct|BreakItemStruct _returnvalue_2)) (.BagMaterial (Utilities|Struct|BreakItemStruct _returnvalue_2)))))))
  (Actor|DestroyActor))

(event EventBeginPlay
  (bind _rotationvalue (Timeline|Timeline_0 Play)
    (:Update
      (Transformation|SetRelativeRotation (Variables|Default|GetScene) (Math|Rotator|MakeRotator 0.0 0.0 _rotationvalue) false false))
    (:Finished
      (Timeline|Timeline_0 PlayFromStart))))

(fn ConstructionScript)