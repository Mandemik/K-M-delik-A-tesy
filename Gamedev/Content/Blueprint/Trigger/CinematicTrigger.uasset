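; Trigger actor that plays a Level Sequence cinematic when the player's ThirdPersonCharacter enters its box.
; The box overlap passes through a DoOnce, stores the player reference and calls StartCinematic.
; StartCinematic creates a sequence player with movement input disabled and HUD hidden, plays it, and binds a finish event.
; The AnimationFinished event is empty, so no follow-up logic runs there.
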(event OnComponentBeginOverlap(Box)
  (params (OverlappedComponent :type Primitive%20Component%20Object%20Reference) (OtherActor :type Actor%20Object%20Reference) (OtherComp :type Primitive%20Component%20Object%20Reference) (OtherBodyIndex :type Integer) (bFromSweep :type Boolean) (SweepResult :type Hit%20Result%20Structure%20%28by%20ref%29))
  (bind _asthird_person_character (Utilities|Casting|CastToThirdPersonCharacter OtherActor))
  (Utilities|FlowControl|DoOnce false
    (:Completed
      (Variables|Default|SetRefToPlayer _asthird_person_character)
      (CallFunction|StartCinematic))))

(event Custom|AnimationFinished)

(event EventBeginPlay)

(event Collision|EventActorBeginOverlap
  (params (OtherActor :type Actor%20Object%20Reference)))

(event EventTick
  (params (DeltaSeconds :type Float%20%28single-precision%29)))

(fn ConstructionScript)

(fn StartCinematic
  (bind _outactor (Sequencer|Player|CreateLevelSequencePlayer (Variables|Default|GetCinematic) (Utilities|Struct|MakeMovieSceneSequencePlaybackSettings false "(Value=0)" 1.0 0.0 false false true false false true false false)))
  (Sequencer|Player|Play (Variables|/Script/LevelSequence.LevelSequenceActor|GetSequencePlayer _outactor) :!class /Script/MovieScene.MovieSceneSequencePlayer)
  (EventDispatchers|BindEventtoOnFinished (Variables|/Script/LevelSequence.LevelSequenceActor|GetSequencePlayer _outactor) (EventDispatchers|CreateEvent :!event Custom|AnimationFinished)))