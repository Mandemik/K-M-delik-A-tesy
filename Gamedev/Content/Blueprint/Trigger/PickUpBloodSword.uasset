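; Blood sword pickup trigger that starts a cinematic, judging by its name and its override of the parent's StartCinematic.
; A looping timeline started on BeginPlay continuously drives the pitch of the Scene component.
; StartCinematic runs the parent logic, sets the player's walk speed and uses SimpleMoveToLocation on the player controller to walk them to the PlayerPlaceToPick point.
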(event EventBeginPlay
  (bind _rotationvalue (Timeline|Timeline_0 Play)
    (:Update
      (Transformation|SetRelativeRotation (Variables|Default|GetScene) (Math|Rotator|MakeRotator 0.0 _rotationvalue 0.0) false false))
    (:Finished
      (Timeline|Timeline_0 PlayFromStart))))

(event EventStartCinematic
  (|CallParentFunction)
  (Variables|/Script/Engine.CharacterMovementComponent|SetMaxWalkSpeed (Variables|/Script/Engine.Character|GetCharacterMovement (Variables|Default|GetRefToPlayer)) 3e+02)
  (AI|Navigation|SimpleMovetoLocation (Game|GetPlayerController 0) (Transformation|GetWorldLocation (Variables|Default|GetPlayerPlaceToPick))))

(fn ConstructionScript
  (|CallParentFunction))